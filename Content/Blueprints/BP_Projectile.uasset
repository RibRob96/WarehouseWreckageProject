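; BP_Projectile is a projectile actor that destroys itself five seconds after BeginPlay.
; Its Launch function applies a single large physics impulse to the static mesh along the mesh's forward vector, scaled by mass since velocity change is off.
; A separate PrintYourName function prints the actor's display name, and neither function is called within this Blueprint.
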(event EventBeginPlay
  (Utilities|FlowControl|Delay 5.0)
  (Actor|DestroyActor))

(event Collision|EventActorBeginOverlap
  (params (OtherActor :type Actor%20Object%20Reference)))

(event EventTick
  (params (DeltaSeconds :type Float%20%28single-precision%29)))

(fn ConstructionScript)

(fn Launch
  (bind _self self)
  (bind _staticmeshcomponent (Variables|Debug|GetStaticMeshComponent _self))
  (Physics|AddImpulse _staticmeshcomponent (* (Math|Vector|GetForwardVector _staticmeshcomponent) 1.5e+06) "None" false))

(fn PrintYourName
  (Development|PrintString (Utilities|GetDisplayName self)))